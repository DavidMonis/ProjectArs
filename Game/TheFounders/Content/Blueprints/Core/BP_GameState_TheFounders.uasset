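; Game state for The Founders that sets up the HUD and holds auto-generated Brick and People resource counters.
; On BeginPlay it creates W_HUD with a reference to itself, adds it to the viewport and switches input to game-and-UI mode.
; It also starts a looping one-second timer, apparently bound to the auto-gen function that increments both counters, with Tick left unused.
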(event EventBeginPlay
  (bind _returnvalue (Game|GetPlayerController 0))
  (Development|PrintString "Create HUD")
  (bind _returnvalue_2 (UserInterface|CreateWidget "/Game/UI/W_HUD.W_HUD_C" _returnvalue self))
  (UserInterface|Viewport|AddtoViewport _returnvalue_2 0)
  (Input|SetInputModeGameandUI _returnvalue _returnvalue_2 "DoNotLock" false false)
  (Utilities|Time|SetTimerbyEvent (EventDispatchers|CreateEvent :!event BPGameStatetheFoundersAutoGenFunc) 1.0 true))

(event EventTick
  (params (DeltaSeconds :type Float%20%28single-precision%29)))

(fn ConstructionScript)

(fn BPGameStatetheFoundersAutoGenFunc
  (Variables|Default|SetBrick (+ (Variables|Default|GetBrick) 1))
  (Variables|Default|SetPeople (+ (Variables|Default|GetPeople) 1)))